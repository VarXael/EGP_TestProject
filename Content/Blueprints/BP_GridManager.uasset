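; BP_GridManager builds a grid of numbered BP_PlacedGrid tiles at BeginPlay and manages the prefabs placed on them, starting with one on tile 0.
; Prefabs spawn by ID from GridToSpawn at a tile's transform, and occupied tiles are refused.
; A downward object trace from the player finds the current tile, printed every tick and used to look up its prefab.
; It can also spawn a BP_CombatGrid linked back to itself.
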(event `self.ReceiveBeginPlay`
  (bind _asbp_character (cast `/Game/Blueprints/BP_Character` (`GameplayStatics.GetPlayerPawn` 0)))
  (set `self.PlayerRef` _asbp_character)
  (`self.SpawnGrid`)
  (`self.SpawnPrefabInGrid` 0))

(event `self.ReceiveTick`
  (params (DeltaSeconds :type "Float (single-precision)"))
  (`KismetSystemLibrary.PrintString` (`KismetStringLibrary.Conv_IntToString` (`self.GetPlayerPosOnGrid`)) true true (struct :`G` 0.66 :`B` 1.0 :`A` 1.0) DeltaSeconds))

(fn `GetGridNumberFromCoordinates`
  (params (X :type Integer) (Y :type Integer))
  (returns (GridNumber :type Integer))
  (return (+ (* X (`self.MaxX`)) Y)))

(fn `GetGridPiece`
  (params (GridNumber :type Integer))
  (returns (GridPieceRef :type "/Game/Blueprints/BP_PlacedGrid Object Reference"))
  (return (`|GetArrayItem` (`self.GridPieceRef`) GridNumber)))

(fn `GetGridPrefabOnPlayerPos`
  (returns (PrefabPlayerIsStandingOn :type "/Game/Blueprints/GridPrefabs/BP_GridPrefab Object Reference"))
  (return (`/Game/Blueprints/BP_PlacedGrid.PiecePlacedOnMe` (`self.GetGridPiece` (`self.GetPlayerPosOnGrid`)))))

(fn `GetPlayerPosOnGrid`
  (returns (PlayerPos :type Integer))
  (bind _capsulecomponent (`Character.CapsuleComponent` (`self.PlayerRef`)))
  (bind (_returnvalue_x _returnvalue_y _returnvalue_z) (`KismetMathLibrary.BreakVector` (`SceneComponent.K2_GetComponentLocation` _capsulecomponent)))
  (bind _outhit (`KismetSystemLibrary.LineTraceSingleForObjects` :`Start` (`SceneComponent.K2_GetComponentLocation` _capsulecomponent) :`End` (`KismetMathLibrary.MakeVector` _returnvalue_x _returnvalue_y (- _returnvalue_z 1000.0)) :`ObjectTypes` (`self.Object Types`) :`DrawDebugType` "ForOneFrame" :`DrawTime` (`GameplayStatics.GetWorldDeltaSeconds`)))
  (bind _asbp_placed_grid (cast `/Game/Blueprints/BP_PlacedGrid` (`.HitActor` (`GameplayStatics.BreakHitResult` _outhit))))
  (return (`/Game/Blueprints/BP_PlacedGrid.GridNumber` _asbp_placed_grid)))

(fn `SetGridCamera`
  (`GameplayStatics.GetActorOfClass` "/Game/Blueprints/BP_CameraManager.BP_CameraManager_C"))

(fn `SpawnCombatArea`
  (returns (CombatArena :type "/Game/Blueprints/BP_CombatGrid Object Reference"))
  (bind _returnvalue (`|SpawnActorFromClass` "/Game/Blueprints/BP_CombatGrid.BP_CombatGrid_C" (`KismetMathLibrary.MakeTransform` (1000.0 1000.0 0.0)) "Undefined" "OverrideRootScale" null null))
  (set `/Game/Blueprints/BP_CombatGrid.GridManagerRef` self _returnvalue)
  (return _returnvalue))

(fn `SpawnGrid`
  (bind _gridpieceref (`self.GridPieceRef`))
  (bind _returnvalue (`KismetMathLibrary.Conv_IntToDouble` (`self.GridPieceSize`)))
  (for _index (range (+ (`self.MaxY`) 1))
    (for _index_2 (range (+ (`self.MaxX`) 1))
      (bind _returnvalue_2 (`|SpawnActorFromClass` "/Game/Blueprints/BP_PlacedGrid.BP_PlacedGrid_C" (`KismetMathLibrary.MakeTransform` (`KismetMathLibrary.MakeVector` (* (`KismetMathLibrary.Conv_IntToDouble` _index) _returnvalue) (* _returnvalue (`KismetMathLibrary.Conv_IntToDouble` _index_2)))) "Undefined" "OverrideRootScale" null null))
      (bind _returnvalue_3 (`KismetArrayLibrary.Array_Add` _gridpieceref _returnvalue_2))
      (set `/Game/Blueprints/BP_PlacedGrid.GridNumber` _returnvalue_3 (`|GetArrayItem` _gridpieceref _returnvalue_3)))))

(fn `SpawnGridPrefab`
  (params (PrefabToSpawnID :type Integer) (GridPieceRef :type "/Game/Blueprints/BP_PlacedGrid Object Reference") (SpawnTransform :type "Transform Structure"))
  (returns (`AsBP Grid Prefab` :type "/Game/Blueprints/GridPrefabs/BP_GridPrefab Object Reference"))
  (bind _returnvalue (`|SpawnActorFromClass` (`|GetArrayItem` (`self.GridToSpawn`) PrefabToSpawnID) SpawnTransform "Undefined" "OverrideRootScale" null null))
  (bind _asbp_grid_prefab (cast `/Game/Blueprints/GridPrefabs/BP_GridPrefab` _returnvalue)
    (:`then`
      (set `/Game/Blueprints/BP_PlacedGrid.PiecePlacedOnMe` _asbp_grid_prefab GridPieceRef)
      (return _asbp_grid_prefab))
    (:`CastFailed`
      (`KismetSystemLibrary.PrintString` "ERROR: Prefab to spawn doesn't exist!" true true (struct :`R` 1.0 :`B` 0.047706 :`A` 1.0)))))

(fn `SpawnPrefabInGrid`
  (params (GridPieceRef :type Integer) (PrefabToSpawnID :type Integer))
  (bind _gridpieceref (`self.GetGridPiece` GridPieceRef))
  (bind (_returnvalue_location _returnvalue_rotation) (`KismetMathLibrary.BreakTransform` (`SceneComponent.K2_GetComponentToWorld` (`/Game/Blueprints/BP_PlacedGrid.Plane` _gridpieceref))))
  (`/Engine/EditorBlueprintResources/StandardMacros.IsValid` (`/Game/Blueprints/BP_PlacedGrid.PiecePlacedOnMe` _gridpieceref)
    (:`Is Valid`
      (`KismetSystemLibrary.PrintString` "Already Has Piece" true true (struct :`R` 1.0 :`G` 0.030402 :`A` 1.0)))
    (:`Is Not Valid`
      (`self.SpawnGridPrefab` PrefabToSpawnID _gridpieceref (`KismetMathLibrary.MakeTransform` _returnvalue_location _returnvalue_rotation)))))

(fn `UserConstructionScript`)