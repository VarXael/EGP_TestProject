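; BP_Character is the player character, which moves on input axes and places the selected card on grid objects by mouse click.
; Number keys 1-3 set the current card ID and update the card widget created, alongside a health bar, at BeginPlay.
; Clicks line-trace from the deprojected cursor, with persistent debug drawing, and pass that ID to the hit BP_PlacedGrid.
; Events fade in the health bar for combat and toggle input during fades.
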(event `self.ReceiveBeginPlay`
  (bind _returnvalue (`GameplayStatics.GetPlayerController` 0))
  (`|ExecutionSequence`
    (:`then_0`
      (bind _returnvalue_2 (`|CreateWidget` "/Game/UI/W_CardUITemporary.W_CardUITemporary_C" _returnvalue))
      (bind _output_get (set `self.UI_CardWidget` _returnvalue_2))
      (`UserWidget.AddToViewport` _output_get 0)
      (set `PlayerController.bShowMouseCursor` true (`GameplayStatics.GetPlayerController` 0)))
    (:`then_1`
      (bind _returnvalue_3 (`|CreateWidget` "/Game/UI/W_HealthBar.W_HealthBar_C" _returnvalue))
      (bind _output_get_2 (set `self.UI_HealthBar` _returnvalue_3))
      (`UserWidget.AddToViewport` _output_get_2 0))))

(event `EnterInCombat`
  (params (Damage :type "Float (double-precision)"))
  (`/Game/UI/W_HealthBar.FadeInAnim` (`self.UI_HealthBar`) Damage))

(event `EnterFadeAnim`
  (`self.DisableInput` (`GameplayStatics.GetPlayerController` 0)))

(event `ExitFadeAnim`
  (`self.EnableInput` (`GameplayStatics.GetPlayerController` 0)))

(event `Key|LeftMouseButton`
  (params (Key :type "Key Structure"))
  (bind (_worldlocation _worlddirection) (`PlayerController.DeprojectMousePositionToWorld` (`GameplayStatics.GetPlayerController` 0)))
  (:`Pressed`
    (bind _outhit (`KismetSystemLibrary.LineTraceSingleForObjects` :`Start` _worldlocation :`End` (+ _worldlocation (* _worlddirection 10000.0)) :`ObjectTypes` (`self.Object Types`) :`DrawDebugType` "Persistent"))
    (bind _asbp_placed_grid (cast `/Game/Blueprints/BP_PlacedGrid` (`.HitActor` (`GameplayStatics.BreakHitResult` _outhit))))
    (`/Game/Blueprints/BP_PlacedGrid.OnCardPlaced` _asbp_placed_grid (`self.CurrentCard ID`))))

(event `InputAxis|Vertical`
  (params (AxisValue :type "Float (single-precision)"))
  (set `self.Vertical` AxisValue)
  (`self.AddMovementInput` (`KismetMathLibrary.MakeVector` (`self.Vertical`) (`self.Horizontal`)) :!label _label))

(event `InputAxis|Horizontal`
  (params (AxisValue :type "Float (single-precision)"))
  (set `self.Horizontal` AxisValue)
  (goto _label))

(event `Key|One`
  (params (Key :type "Key Structure"))
  (:`Pressed`
    (set `self.CurrentCard ID` 0)
    (`/Game/UI/W_CardUITemporary.ChangeCard` (`self.UI_CardWidget`) (`self.CurrentCard ID`) :!label _label_2)))

(event `Key|Two`
  (params (Key :type "Key Structure"))
  (:`Pressed`
    (set `self.CurrentCard ID` 1)
    (goto _label_2)))

(event `Key|Three`
  (params (Key :type "Key Structure"))
  (:`Pressed`
    (set `self.CurrentCard ID` 2)
    (goto _label_2)))

(fn `DecreaseHealthBar`
  (params (Damage :type "Float (double-precision)"))
  (set `self.CurrentHealth` (- (`self.CurrentHealth`) Damage))
  (return))

(fn `UserConstructionScript`)