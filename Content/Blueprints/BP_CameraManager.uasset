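; Camera manager that spawns a BP_Camera as the view target and moves it to the CameraPos of the grid piece the player occupies.
; Tick compares the player's cell from BP_GridManager with the current one and resumes a looping SwitchCamera timer on change.
; The timer feeds accumulated time into VInterpTo as DeltaTime, so the pull strengthens each step, and pauses itself on arrival.
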(event `self.ReceiveBeginPlay`
  (`|ExecutionSequence`
    (:`then_0`
      (`self.SpawnCamera`)
      (bind _returnvalue (`GameplayStatics.GetActorOfClass` "/Game/Blueprints/BP_GridManager.BP_GridManager_C"))
      (set `self.GridManagerRef` _returnvalue))
    (:`then_1`
      (bind _returnvalue_2 (`KismetSystemLibrary.K2_SetTimer` null "SwitchCamera" 0.02 true))
      (bind _output_get (set `self.SwitchCameraTimer` _returnvalue_2))
      (`KismetSystemLibrary.K2_UnPauseTimerHandle` _output_get))))

(event `self.ReceiveTick`
  (params (DeltaSeconds :type "Float (single-precision)"))
  (if (!= (`self.CurrentCameraGrid`) (`/Game/Blueprints/BP_GridManager.GetPlayerPosOnGrid` (`self.GridManagerRef`)))
    (set `self.SwitchCameraTime` 0.0)
    (`KismetSystemLibrary.K2_UnPauseTimerHandle` (`self.SwitchCameraTimer`))))

(fn `SpawnCamera`
  (bind _returnvalue (`|SpawnActorFromClass` "/Game/Blueprints/BP_Camera.BP_Camera_C" (`self.CameraSpawnPoint`) "Undefined" "OverrideRootScale" null null))
  (bind _output_get (set `self.CameraRef` _returnvalue))
  (`PlayerController.SetViewTargetWithBlend` (`GameplayStatics.GetPlayerController` 0) _output_get 0.0 "VTBlend_Linear" 0.0 false))

(fn `SwitchCamera`
  (bind _gridmanagerref (`self.GridManagerRef`))
  (bind _defaultsceneroot (`/Game/Blueprints/BP_Camera.DefaultSceneRoot` (`self.CameraRef`)))
  (bind _camerapos (`/Game/Blueprints/BP_PlacedGrid.CameraPos` (`/Game/Blueprints/BP_GridManager.GetGridPiece` _gridmanagerref (`/Game/Blueprints/BP_GridManager.GetPlayerPosOnGrid` _gridmanagerref))))
  (set `self.CurrentCameraGrid` (`/Game/Blueprints/BP_GridManager.GetPlayerPosOnGrid` (`self.GridManagerRef`)))
  (bind _output_get (set `self.SwitchCameraTime` (+ (`self.SwitchCameraTime`) 0.02)))
  (`SceneComponent.K2_SetWorldLocation` _defaultsceneroot (`KismetMathLibrary.VInterpTo` (`SceneComponent.K2_GetComponentLocation` (`/Game/Blueprints/BP_Camera.DefaultSceneRoot` (`self.CameraRef`))) (`SceneComponent.K2_GetComponentLocation` _camerapos) _output_get 1.0) false true)
  (if (== (`SceneComponent.K2_GetComponentLocation` _defaultsceneroot) (`SceneComponent.K2_GetComponentLocation` _camerapos) :`ErrorTolerance` 0.1)
    (set `self.SwitchCameraTime` 0.0)
    (`KismetSystemLibrary.K2_PauseTimerHandle` (`self.SwitchCameraTimer`))
    (return)))

(fn `UserConstructionScript`
  (set `self.CameraSpawnPoint` (`SceneComponent.K2_GetComponentToWorld` (`self.CameraPos`))))