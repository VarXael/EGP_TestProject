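; A single grid cell actor that receives placed cards and has the grid manager spawn the matching prefab in that cell.
; On BeginPlay it finds BP_GridManager, scales its Plane to the manager's piece size, and shifts CameraPos back along X and up by that size.
; OnCardPlaced passes the cell's GridNumber and the CardID to SpawnPrefabInGrid, while OnCardHover is an empty stub.
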(event `self.ReceiveBeginPlay`
  (bind (_returnvalue_x _returnvalue_y _returnvalue_z) (`KismetMathLibrary.BreakVector` (`SceneComponent.K2_GetComponentLocation` (`self.CameraPos`))))
  (bind _returnvalue (`GameplayStatics.GetActorOfClass` "/Game/Blueprints/BP_GridManager.BP_GridManager_C"))
  (bind _output_get (set `self.GridReference` _returnvalue))
  (bind _gridpiecesize (`/Game/Blueprints/BP_GridManager.GridPieceSize` _output_get))
  (bind _returnvalue_2 (`KismetMathLibrary.Conv_IntToDouble` (/ _gridpiecesize 100)))
  (`SceneComponent.SetWorldScale3D` (`self.Plane`) (`KismetMathLibrary.MakeVector` _returnvalue_2 _returnvalue_2))
  (bind _returnvalue_3 (`KismetMathLibrary.Conv_IntToDouble` _gridpiecesize))
  (`SceneComponent.K2_SetWorldLocation` (`self.CameraPos`) (`KismetMathLibrary.MakeVector` (- _returnvalue_x _returnvalue_3) _returnvalue_y (+ _returnvalue_3 _returnvalue_z)) false true))

(event `/Game/Blueprints/Interfaces/I_GridInterface.OnCardPlaced`
  (params (CardID :type Integer))
  (`/Game/Blueprints/BP_GridManager.SpawnPrefabInGrid` (`self.GridReference`) (`self.GridNumber`) CardID))

(event `OnCardHover`)

(fn `UserConstructionScript`)